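; Homing tower-defense projectile that chases its EnemyTarget and damages Enemy_Gob actors.
; Tick steers it toward the living target and caches that location; if the target dies while still valid, it flies on to the cached point, or is destroyed if none was stored.
; Overlapping any Enemy_Gob applies damage from the game mode's Tower1 value plus a fixed bonus.
; Hits and arrivals at the cached point play an impact sound before destruction.
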(event `DestroySelf`
  (`self.PlayImpactSound`)
  (`self.K2_DestroyActor`))

(event `self.ReceiveTick`
  (params (DeltaSeconds :type "Float (single-precision)"))
  (bind _enemytarget (`self.EnemyTarget`))
  (bind _returnvalue (`self.K2_GetActorLocation` _enemytarget))
  (bind _returnvalue_2 (* DeltaSeconds (`self.Speed`)))
  (`/Engine/EditorBlueprintResources/StandardMacros.IsValid` _enemytarget
    (:`Is Valid`
      (if (`/Game/TowerDefense/Blueprints/Enemy_Gob.isAlive` _enemytarget)
        (`self.K2_AddActorWorldOffset` (* (`KismetMathLibrary.Normal` (- _returnvalue (`self.K2_GetActorLocation`))) _returnvalue_2))
        (`/Engine/EditorBlueprintResources/StandardMacros.IsValid` _enemytarget
          (:`Is Valid`
            (set `self.TargetLocation` _returnvalue)))
        (elif (== (`self.TargetLocation`) (0.0 0.0 0.0) :`ErrorTolerance` 5.0)
          (`self.K2_DestroyActor`)
          (else
            (`self.K2_AddActorWorldOffset` (* (`KismetMathLibrary.Normal` (- (`self.TargetLocation`) (`self.K2_GetActorLocation`))) _returnvalue_2))
            (if (== (`self.K2_GetActorLocation`) (`self.TargetLocation`) :`ErrorTolerance` 20.0)
              (`self.DestroySelf`))))))))

(event `self.Bullet.OnComponentBeginOverlap`
  (params (OverlappedComponent :type "PrimitiveComponent Object Reference") (OtherActor :type "Actor Object Reference") (OtherComp :type "PrimitiveComponent Object Reference") (OtherBodyIndex :type Integer) (bFromSweep :type Boolean) (SweepResult :type "HitResult Structure (by ref)"))
  (bind _asenemy_gob (cast `/Game/TowerDefense/Blueprints/Enemy_Gob` OtherActor))
  (bind _astower_defense_game_mode (cast `/Game/TowerDefense/Blueprints/TowerDefenseGameMode` (`GameplayStatics.GetGameMode`)))
  (`/Game/TowerDefense/Blueprints/Enemy_Gob.TakeDamage` _asenemy_gob (+ (`/Game/TowerDefense/Blueprints/TowerDefenseGameMode.Tower1` _astower_defense_game_mode) 3.0))
  (`self.DestroySelf`))

(event `PlayImpactSound`
  (`GameplayStatics.PlaySoundAtLocation` (`self.ImpactSound`) (`self.K2_GetActorLocation`)))

(fn `UserConstructionScript`)