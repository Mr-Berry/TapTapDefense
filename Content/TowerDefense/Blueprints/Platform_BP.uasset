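; Clickable tower defense platform that opens a tower selection or sell/upgrade menu.
; On BeginPlay it adds two manually attached widget components at the Scene's world transform, enlarges the upgrade one, and passes itself to their TowerSelection and Sell widgets.
; Clicking the cube checks BlockState, showing the tower selection widget when it is zero and the upgrade widget otherwise.
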(event `self.ReceiveBeginPlay`
  (bind _returnvalue (`AddComponent|NODE_AddWidgetComponent-0` :`bManualAttachment` true :`RelativeTransform` (`SceneComponent.K2_GetComponentToWorld` (`self.Scene`))))
  (set `self.TowerWidget` _returnvalue)
  (bind _astower_selection (cast `/Game/TowerDefense/Interface/TowerSelection` (`WidgetComponent.GetUserWidgetObject` _returnvalue)))
  (set `/Game/TowerDefense/Interface/TowerSelection.Platform` self _astower_selection)
  (bind _returnvalue_2 (`AddComponent|NODE_AddWidgetComponent-1` :`bManualAttachment` true :`RelativeTransform` (`SceneComponent.K2_GetComponentToWorld` (`self.Scene`))))
  (bind _output_get (set `self.UpgradeWidget` _returnvalue_2))
  (`SceneComponent.SetRelativeScale3D` _output_get (3.0 3.0 3.0))
  (bind _assell (cast `/Game/TowerDefense/Interface/Sell` (`WidgetComponent.GetUserWidgetObject` _returnvalue_2)))
  (set `/Game/TowerDefense/Interface/Sell.Platform` self _assell))

(event `self.Cube.OnClicked`
  (params (TouchedComponent :type "PrimitiveComponent Object Reference") (ButtonPressed :type "Key Structure" :default "AnyKey"))
  (if (== (`self.BlockState`) 0)
    (`SceneComponent.SetVisibility` (`self.TowerWidget`) true false)
    (else
      (`SceneComponent.SetVisibility` (`self.UpgradeWidget`) true false))))

(fn `UserConstructionScript`)