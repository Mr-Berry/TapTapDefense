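; Tower defense game mode that runs enemy spawning, fame, gold, combo scoring and save/load.
; A looping timer spawns goblins, with periodic vampires and bosses, at random spawn points and aims their AI at a waypoint.
; Fame level-ups shorten the spawn interval and scale enemy health, while combo level feeds an enemy multiplier and decays on a timer.
; Saves store progress and platform states, and loading respawns turrets on platform sockets.
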(event `self.ReceiveBeginPlay`
  (bind _outactors (`GameplayStatics.GetAllActorsOfClass` "/Game/TowerDefense/Blueprints/SpawnPoint.SpawnPoint_C"))
  (set `self.SpawnPoints` _outactors))

(event `self.ReceiveTick`
  (params (DeltaSeconds :type "Float (single-precision)"))
  (bind _returnvalue (/ 5.0 (`KismetMathLibrary.Conv_IntToDouble` (+ (`self.FameLevel`) 1))))
  (if (`self.Increment`)
    (set `self.Increment` false)
    (if (>= _returnvalue 0.5)
      (set `self.SpawnTime` _returnvalue)
      (else
        (set `self.SpawnTime` 0.5)))
    (`KismetSystemLibrary.K2_ClearTimer` null "SpawnNewEnemy")
    (`KismetSystemLibrary.K2_SetTimer` null "SpawnNewEnemy" (`self.SpawnTime`) true)))

(event `SpawnEnemy`
  (`self.SpawnNewEnemy`))

(event `Combo++`
  (`KismetSystemLibrary.K2_ClearTimer` null "ComboDecrement")
  (`self.ComboIncrement`)
  (`self.ComboLevelIncrement`)
  (`self.SetComboTotal`)
  (`KismetSystemLibrary.Delay` 10.0)
  (`self.Combo--`))

(event `Combo--`
  (`KismetSystemLibrary.K2_SetTimer` null "ComboDecrement" 1.0 true))

(event `EnemyDeath`
  (params (FameAwarded :type Integer))
  (`self.Fame++` FameAwarded)
  (set `self.Gold` (+ (* FameAwarded 2) (`self.Gold`))))

(event `Fame++`
  (params (FameAwarded :type Integer))
  (set `self.Fame` (+ FameAwarded (`self.Fame`)))
  (`self.FameLevelIncrement`))

(event `Fame--`
  (params (FameLost :type Integer))
  (set `self.Fame` (- (`self.Fame`) (* (+ FameLost (`self.FameLevel`)) 2)))
  (`self.FameLevelDecrement`))

(event `SaveGame`
  (bind _savedata (`self.SaveData`))
  ;[1 1 1] SaveGame
  (set `/Game/TowerDefense/Interface/SaveData.FameLevel` (`self.FameLevel`) _savedata)
  (set `/Game/TowerDefense/Interface/SaveData.MaxFameLevel` (`self.HighestFameReached`) _savedata)
  (set `/Game/TowerDefense/Interface/SaveData.Fame` (`self.Fame`) _savedata)
  (set `/Game/TowerDefense/Interface/SaveData.Tower_0` (`self.Tower1`) _savedata)
  (set `/Game/TowerDefense/Interface/SaveData.Tower_1` (`self.Tower2`) _savedata)
  (set `/Game/TowerDefense/Interface/SaveData.Tower_2` (`self.Tower3`) _savedata)
  (set `/Game/TowerDefense/Interface/SaveData.FameMax` (`self.FameMax`) _savedata)
  (set `/Game/TowerDefense/Interface/SaveData.Gold` (`self.Gold`) _savedata)
  (bind _platformstates (`self.GetplatformStates`))
  (set `/Game/TowerDefense/Interface/SaveData.PlatformStates` _platformstates _savedata)
  (`GameplayStatics.SaveGameToSlot` _savedata "Save"))

(event `LoadGame`
  (bind _savedata (`self.SaveData`))
  ;[1 1 1] LoadGame
  (set `self.Fame` (`/Game/TowerDefense/Interface/SaveData.Fame` _savedata))
  (set `self.FameLevel` (`/Game/TowerDefense/Interface/SaveData.FameLevel` _savedata))
  (set `self.HighestFameReached` (`/Game/TowerDefense/Interface/SaveData.MaxFameLevel` _savedata))
  (set `self.FameMax` (`/Game/TowerDefense/Interface/SaveData.FameMax` _savedata))
  (set `self.Gold` (`/Game/TowerDefense/Interface/SaveData.Gold` _savedata))
  (set `self.Tower1` (`/Game/TowerDefense/Interface/SaveData.Tower_0` _savedata))
  (set `self.Tower2` (`/Game/TowerDefense/Interface/SaveData.Tower_1` _savedata))
  (set `self.Tower3` (`/Game/TowerDefense/Interface/SaveData.Tower_2` _savedata))
  (`self.SetPlatformStates` (`/Game/TowerDefense/Interface/SaveData.PlatformStates` _savedata)))

(fn `ComboDecrement`
  (bind _combolevel (`self.ComboLevel`))
  (if (>= _combolevel 3)
    (set `self.Combo` (- (`self.Combo`) (* _combolevel 2)))
    (else
      (set `self.Combo` (- (`self.Combo`) 5))))
  (`self.ComboLevelIncrement`)
  (`self.SetComboTotal`)
  (`self.ComboZeroed`))

(fn `ComboIncrement`
  (bind _combolevel (`self.ComboLevel`))
  (if (> _combolevel 2)
    (set `self.Combo` (+ (`self.Combo`) _combolevel))
    (else
      (set `self.Combo` (+ (`self.Combo`) 2)))))

(fn `ComboLevelIncrement`
  (bind _combo (`self.Combo`))
  (if (>= _combo 50)
    (`/Engine/EditorBlueprintResources/StandardMacros.IncrementInt` (`self.ComboLevel`)
      (:`  `
        (set `self.Combo` 0)))
    (elif (<= _combo 0)
      (`/Engine/EditorBlueprintResources/StandardMacros.DecrementInt` (`self.ComboLevel`)
        (:`  `
          (set `self.Combo` 49))))))

(fn `ComboZeroed`
  (if (and (<= (`self.ComboTotal`) 0) (<= (`self.ComboLevel`) 0))
    (set `self.Combo` 0)
    (set `self.ComboLevel` 0)
    (set `self.ComboTotal` 0)
    (`KismetSystemLibrary.K2_ClearTimer` null "ComboDecrement")))

(fn `FameLevelDecrement`
  (if (<= (`self.Fame`) 0)
    (if (<= (`self.FameLevel`) 0)
      (set `self.Fame` 0)
      (else
        (bind _output_get (set `self.FameMax` (`KismetMathLibrary.FTrunc` (/ (`KismetMathLibrary.Conv_IntToDouble` (`self.FameMax`)) 1.5))))
        (set `self.Fame` (- _output_get 1))
        (`/Engine/EditorBlueprintResources/StandardMacros.DecrementInt` (`self.FameLevel`))))))

(fn `FameLevelIncrement`
  (bind _famemax (`self.FameMax`))
  (if (>= (`self.Fame`) _famemax)
    (`/Engine/EditorBlueprintResources/StandardMacros.IncrementInt` (`self.FameLevel`)
      (:`  `
        (set `self.Fame` 0)
        (set `self.FameMax` (`KismetMathLibrary.FTrunc` (* _famemax 1.5)))
        (set `self.Increment` true)))))

(fn `GetplatformStates`
  (returns (PlatformStates :type "Array of Integer"))
  (bind _platformstates (`self.PlatformStates`))
  (bind _outactors (`GameplayStatics.GetAllActorsOfClass` "/Game/TowerDefense/Blueprints/Platform_BP.Platform_BP_C"))
  (for _array_element _outactors
    (`KismetArrayLibrary.Array_Add` _platformstates (`/Game/TowerDefense/Blueprints/Platform_BP.BlockState` _array_element)))
  (return _platformstates))

(fn `GetSpawnEnemyIndex`
  (returns (EnemyIndex :type Integer))
  (locals (RetVal :type Integer))
  (bind _spawnedcount (`self.SpawnedCount`))
  (bind _returnvalue (!= _spawnedcount 0))
  (if (and (== (mod _spawnedcount 15) 0) _returnvalue)
    (set `local.RetVal` 2)
    (elif (and (== (mod _spawnedcount 5) 0) _returnvalue)
      (set `local.RetVal` 1)))
  (return (`local.RetVal`)))

(fn `GetTargetPosition`
  (params (Enemy :type "/Game/TowerDefense/Blueprints/Enemy_Gob Object Reference") (WPodd :type "TargetPoint Object Reference") (WPeven :type "TargetPoint Object Reference"))
  (returns (Target :type "Vector Structure"))
  (locals (TargetRet :type "Vector Structure"))
  (bind _z (.z (`self.K2_GetActorLocation` Enemy)))
  (`/Engine/EditorBlueprintResources/StandardMacros.IsValid` WPodd
    (:`Is Valid`
      (set `local.TargetRet` (`KismetMathLibrary.MakeVector` (.x (`self.K2_GetActorLocation` WPodd)) (.y (`self.K2_GetActorLocation` Enemy)) _z)))
    (:`Is Not Valid`
      (set `local.TargetRet` (`KismetMathLibrary.MakeVector` (.x (`self.K2_GetActorLocation` Enemy)) (.y (`self.K2_GetActorLocation` WPeven)) _z))))
  (return (`local.TargetRet`)))

(fn `SetComboTotal`
  (set `self.ComboTotal` (+ (`self.Combo`) (* (`self.ComboLevel`) 50))))

(fn `SetPlatformStates`
  (params (PlatformStates :type "Array of Integer"))
  (locals (i :type Integer))
  (bind _i (`local.i`))
  (bind _outactors (`GameplayStatics.GetAllActorsOfClass` "/Game/TowerDefense/Blueprints/Platform_BP.Platform_BP_C"))
  (for _array_element _outactors
    (bind _output_get (set `/Game/TowerDefense/Blueprints/Platform_BP.BlockState` (`|GetArrayItem` PlatformStates _i) _array_element))
    (`/Engine/EditorBlueprintResources/StandardMacros.IncrementInt` _i
      (:`  `
        (switch `int` _output_get
          (:`1`
            (`self.SpawnAndAttachTurret` _array_element))
          (:`2`
            (`self.SpawnAndAttachAoe` _array_element))
          (:`3`
            (`self.SpawnAndAttachLaser` _array_element)))))))

(fn `SpawnAndAttachAoe`
  (params (Platform :type "/Game/TowerDefense/Blueprints/Platform_BP Object Reference"))
  (bind _returnvalue (`|SpawnActorFromClass` "/Game/TowerDefense/Blueprints/AoETurret.AoETurret_C" (`KismetMathLibrary.MakeTransform` (0.0 0.0 0.0)) "AlwaysSpawn" "OverrideRootScale"))
  (`self.K2_AttachToComponent` _returnvalue (`StaticMeshActor.StaticMeshComponent` Platform) "explosiveTurret" "SnapToTarget" "SnapToTarget" "SnapToTarget" true))

(fn `SpawnAndAttachLaser`
  (params (platform :type "/Game/TowerDefense/Blueprints/Platform_BP Object Reference"))
  (bind _returnvalue (`|SpawnActorFromClass` "/Game/TowerDefense/Blueprints/LaserTurret.LaserTurret_C" (`KismetMathLibrary.MakeTransform` (0.0 0.0 0.0)) "AlwaysSpawn" "OverrideRootScale"))
  (`self.K2_AttachToComponent` _returnvalue (`StaticMeshActor.StaticMeshComponent` platform) "laserTurret" "SnapToTarget" "SnapToTarget" "SnapToTarget" true))

(fn `SpawnAndAttachTurret`
  (params (Platform :type "/Game/TowerDefense/Blueprints/Platform_BP Object Reference"))
  (bind _returnvalue (`|SpawnActorFromClass` "/Game/TowerDefense/Blueprints/BasicTurret.BasicTurret_C" (`KismetMathLibrary.MakeTransform` (0.0 0.0 0.0)) "AlwaysSpawn" "OverrideRootScale"))
  (`self.K2_AttachToComponent` _returnvalue (`StaticMeshActor.StaticMeshComponent` Platform) "basicTurret" "SnapToTarget" "SnapToTarget" "SnapToTarget" true))

(fn `SpawnBoss`
  (params (Location :type "Vector Structure"))
  (bind _returnvalue (`|SpawnActorFromClass` "/Game/TowerDefense/Blueprints/Enemy_Boss.Enemy_Boss_C" (`KismetMathLibrary.MakeTransform` Location (struct) (1.3 1.3 1.3)) "AlwaysSpawn" "OverrideRootScale"))
  (`/Game/TowerDefense/Blueprints/Enemy_Gob.SetParamters` _returnvalue 10.0 5 (`KismetMathLibrary.Conv_IntToDouble` (+ (`self.ComboLevel`) 1)) (`KismetMathLibrary.Conv_IntToDouble` (* (+ (`self.FameLevel`) 1) 2)))
  (bind _target (`self.GetTargetPosition` _returnvalue (`self.WayPoint1`)))
  (bind _asaic_bp (cast `/Game/TowerDefense/Blueprints/AIC_BP` (`AIBlueprintHelperLibrary.GetAIController` _returnvalue)))
  (set `/Game/TowerDefense/Blueprints/AIC_BP.Target` _target _asaic_bp))

(fn `SpawnGob`
  (params (location :type "Vector Structure"))
  (bind _returnvalue (`|SpawnActorFromClass` "/Game/TowerDefense/Blueprints/Enemy_Gob.Enemy_Gob_C" (`KismetMathLibrary.MakeTransform` location (struct) (0.5 0.5 0.5)) "AlwaysSpawn" "OverrideRootScale"))
  (`/Game/TowerDefense/Blueprints/Enemy_Gob.SetParamters` _returnvalue 2.0 1 (`KismetMathLibrary.Conv_IntToDouble` (+ (`self.ComboLevel`) 1)) (`KismetMathLibrary.Conv_IntToDouble` (* (+ (`self.FameLevel`) 1) 2)))
  (bind _target (`self.GetTargetPosition` _returnvalue (`self.WayPoint1`)))
  (bind _asaic_bp (cast `/Game/TowerDefense/Blueprints/AIC_BP` (`AIBlueprintHelperLibrary.GetAIController` _returnvalue)))
  (set `/Game/TowerDefense/Blueprints/AIC_BP.Target` _target _asaic_bp))

(fn `SpawnNewEnemy`
  (bind _returnvalue (`self.K2_GetActorLocation` (`|GetArrayItem` (`self.SpawnPoints`) (`KismetMathLibrary.RandomInteger` 5))))
  (bind _enemyindex (`self.GetSpawnEnemyIndex`))
  (switch `int` _enemyindex
    (:`Default`
      (`self.SpawnBoss` _returnvalue))
    (:`0`
      (`self.SpawnGob` _returnvalue))
    (:`1`
      (`self.SpawnVamp` _returnvalue)))
  (`/Engine/EditorBlueprintResources/StandardMacros.IncrementInt` (`self.SpawnedCount`)))

(fn `SpawnVamp`
  (params (Location :type "Vector Structure"))
  (bind _returnvalue (`|SpawnActorFromClass` "/Game/TowerDefense/Blueprints/Enemy_Vamp.Enemy_Vamp_C" (`KismetMathLibrary.MakeTransform` Location (struct) (0.9 0.9 0.9)) "AlwaysSpawn" "OverrideRootScale"))
  (`/Game/TowerDefense/Blueprints/Enemy_Gob.SetParamters` _returnvalue 5.0 3 (`KismetMathLibrary.Conv_IntToDouble` (+ (`self.ComboLevel`) 1)) (`KismetMathLibrary.Conv_IntToDouble` (* (+ (`self.FameLevel`) 1) 2)))
  (bind _target (`self.GetTargetPosition` _returnvalue (`self.WayPoint1`)))
  (bind _asaic_bp (cast `/Game/TowerDefense/Blueprints/AIC_BP` (`AIBlueprintHelperLibrary.GetAIController` _returnvalue)))
  (set `/Game/TowerDefense/Blueprints/AIC_BP.Target` _target _asaic_bp))

(fn `UserConstructionScript`)