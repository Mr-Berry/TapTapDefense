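; Area-of-effect tower defense projectile that damages every nearby Enemy_Gob when it hits one.
; An ExplosionRange component keeps the EnemiesInRange list current through begin and end overlaps.
; A Bullet overlap with an enemy calls DestroySelf, which damages each listed enemy by the game mode's Tower2 value plus one.
; It then spawns a scaled-down, sped-up ice shatter effect, plays the impact sound and destroys the actor.
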(event `self.ExplosionRange.OnComponentBeginOverlap`
  (params (OverlappedComponent :type "PrimitiveComponent Object Reference") (OtherActor :type "Actor Object Reference") (OtherComp :type "PrimitiveComponent Object Reference") (OtherBodyIndex :type Integer) (bFromSweep :type Boolean) (SweepResult :type "HitResult Structure (by ref)"))
  (bind _asenemy_gob (cast `/Game/TowerDefense/Blueprints/Enemy_Gob` OtherActor))
  (`KismetArrayLibrary.Array_Add` (`self.EnemiesInRange`) _asenemy_gob))

(event `self.ExplosionRange.OnComponentEndOverlap`
  (params (OverlappedComponent :type "PrimitiveComponent Object Reference") (OtherActor :type "Actor Object Reference") (OtherComp :type "PrimitiveComponent Object Reference") (OtherBodyIndex :type Integer))
  (bind _asenemy_gob (cast `/Game/TowerDefense/Blueprints/Enemy_Gob` OtherActor))
  (`KismetArrayLibrary.Array_RemoveItem` (`self.EnemiesInRange`) _asenemy_gob))

(event `self.BndEvt__Bullet_K2Node_ComponentBoundEvent_0_ComponentBeginOverlapSignature__DelegateSignature`
  (params (OverlappedComponent :type "PrimitiveComponent Object Reference") (OtherActor :type "Actor Object Reference") (OtherComp :type "PrimitiveComponent Object Reference") (OtherBodyIndex :type Integer) (bFromSweep :type Boolean) (SweepResult :type "HitResult Structure (by ref)"))
  (cast `/Game/TowerDefense/Blueprints/Enemy_Gob` OtherActor)
  (`self.DestroySelf` :!label _label))

(event `self.Bullet.OnComponentBeginOverlap`
  (params (OverlappedComponent :type "PrimitiveComponent Object Reference") (OtherActor :type "Actor Object Reference") (OtherComp :type "PrimitiveComponent Object Reference") (OtherBodyIndex :type Integer) (bFromSweep :type Boolean) (SweepResult :type "HitResult Structure (by ref)"))
  (cast `/Game/TowerDefense/Blueprints/Enemy_Gob` OtherActor)
  (goto _label))

(event `self.DestroySelf`
  (bind _astower_defense_game_mode (cast `/Game/TowerDefense/Blueprints/TowerDefenseGameMode` (`GameplayStatics.GetGameMode`)))
  (for _array_element (`self.EnemiesInRange`)
    (`/Game/TowerDefense/Blueprints/Enemy_Gob.TakeDamage` _array_element (+ (`/Game/TowerDefense/Blueprints/TowerDefenseGameMode.Tower2` _astower_defense_game_mode) 1.0)))
  (bind _returnvalue (`GameplayStatics.SpawnEmitterAtLocation` "/Game/TowerDefense/Particle/P_Aura_Ice_Shatter_01.P_Aura_Ice_Shatter_01" (`SceneComponent.K2_GetComponentLocation` (`self.Bullet`)) (struct) false))
  (`SceneComponent.SetWorldScale3D` _returnvalue (0.2 0.2 0.2))
  (set `ParticleSystemComponent.CustomTimeDilation` 2.0 _returnvalue)
  (`self.PlayImpactSound`)
  (`self.K2_DestroyActor`))

(fn `UserConstructionScript`
  (`parent.UserConstructionScript`))