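; Laser turret for the tower defense game that charges up, then fires a beam damaging every Enemy_Gob in its line of fire.
; Range overlaps track enemies, targeting the last in the list, while Tick rotates the head toward it and retargets when it is invalid or dead.
; A looping timer builds charge; once charged and aligned, the beam flashes, damages Box occupants by the GameMode's Tower3 value, then recharges.
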(event `self.ReceiveBeginPlay`
  (`KismetSystemLibrary.K2_SetTimer` null "ChargeUp" 0.1 true))

(event `self.ReceiveTick`
  (params (DeltaSeconds :type "Float (single-precision)"))
  (bind _targetable_ (`self.ValidAndAlive?`))
  (if _targetable_
    (bind _facingtarget_ (`self.RotateToTarget` DeltaSeconds))
    (if (and (`self.Charged`) _facingtarget_)
      (`self.ActivateLaser`)
      (`KismetSystemLibrary.Delay` 1.0)
      (`self.DeactvateLaser`)
      (set `self.Charged` false)
      (set `self.Charge` 0.0)
      (`KismetSystemLibrary.K2_SetTimer` null "ChargeUp" 0.1 true)
      (else
        (`ParticleSystemComponent.SetTemplate` (`self.LaserEmitter`) null)))
    (else
      (`self.ChangeTarget`))))

(event `FireAndKickBack`
  (params (Arrow :type "ArrowComponent Object Reference") (Turret :type "StaticMeshComponent Object Reference"))
  (`/Engine/EditorBlueprintResources/StandardMacros.IsValid` (`self.FarthestEnemy`)
    (:`Is Valid`
      (`self.Fire` Arrow)
      (`KismetSystemLibrary.MoveComponentTo` Turret (0.0 -80.0 0.0) (struct) true false 0.3)
      (`KismetSystemLibrary.MoveComponentTo` Turret (0.0 0.0 0.0) (struct) true false 0.3))))

(event `self.Range.OnComponentBeginOverlap`
  (params (OverlappedComponent :type "PrimitiveComponent Object Reference") (OtherActor :type "Actor Object Reference") (OtherComp :type "PrimitiveComponent Object Reference") (OtherBodyIndex :type Integer) (bFromSweep :type Boolean) (SweepResult :type "HitResult Structure (by ref)"))
  (bind _enemiesinrange (`self.EnemiesInRange`))
  ;[1 1 1] Targets in/ targets out
  (bind _asenemy_gob (cast `/Game/TowerDefense/Blueprints/Enemy_Gob` OtherActor))
  (set `self.enemyInRange` true)
  (`KismetArrayLibrary.Array_Add` _enemiesinrange _asenemy_gob)
  (set `self.FarthestEnemy` (`|GetArrayItem` _enemiesinrange (`KismetArrayLibrary.Array_LastIndex` _enemiesinrange))))

(event `self.Range.OnComponentEndOverlap`
  (params (OverlappedComponent :type "PrimitiveComponent Object Reference") (OtherActor :type "Actor Object Reference") (OtherComp :type "PrimitiveComponent Object Reference") (OtherBodyIndex :type Integer))
  (bind _enemiesinrange (`self.EnemiesInRange`))
  ;[1 1 1] Targets in/ targets out
  (bind _asenemy_gob (cast `/Game/TowerDefense/Blueprints/Enemy_Gob` OtherActor))
  (`KismetArrayLibrary.Array_RemoveItem` _enemiesinrange _asenemy_gob)
  (if (!= (`KismetArrayLibrary.Array_Length` _enemiesinrange) 0)
    (set `self.FarthestEnemy` (`|GetArrayItem` _enemiesinrange (`KismetArrayLibrary.Array_LastIndex` _enemiesinrange)))
    (else
      (set `self.enemyInRange` false))))

(event `self.Box.OnComponentBeginOverlap`
  (params (OverlappedComponent :type "PrimitiveComponent Object Reference") (OtherActor :type "Actor Object Reference") (OtherComp :type "PrimitiveComponent Object Reference") (OtherBodyIndex :type Integer) (bFromSweep :type Boolean) (SweepResult :type "HitResult Structure (by ref)"))
  (bind _asenemy_gob (cast `/Game/TowerDefense/Blueprints/Enemy_Gob` OtherActor))
  (`KismetArrayLibrary.Array_Add` (`self.EnemiesInLineOfFire`) _asenemy_gob))

(event `self.Box.OnComponentEndOverlap`
  (params (OverlappedComponent :type "PrimitiveComponent Object Reference") (OtherActor :type "Actor Object Reference") (OtherComp :type "PrimitiveComponent Object Reference") (OtherBodyIndex :type Integer))
  (bind _asenemy_gob (cast `/Game/TowerDefense/Blueprints/Enemy_Gob` OtherActor))
  (`KismetArrayLibrary.Array_RemoveItem` (`self.EnemiesInLineOfFire`) _asenemy_gob))

(fn `ActivateLaser`
  (bind _laseremitter (`self.LaserEmitter`))
  (bind _arrow (`self.Arrow`))
  (`GameplayStatics.PlaySoundAtLocation` "/Game/TowerDefense/Sounds/Laser_Cue.Laser_Cue" (`self.K2_GetActorLocation`))
  (`ParticleSystemComponent.SetTemplate` _laseremitter "/Game/TowerDefense/Particle/Beam.Beam")
  (`SceneComponent.SetVisibility` _laseremitter true true)
  (`ParticleSystemComponent.SetBeamSourcePoint` _laseremitter 0 (`SceneComponent.K2_GetComponentLocation` _arrow) 0)
  (`ParticleSystemComponent.SetBeamTargetPoint` _laseremitter 0 (* (`SceneComponent.GetForwardVector` _arrow) 1500.0) 0)
  (bind _astower_defense_game_mode (cast `/Game/TowerDefense/Blueprints/TowerDefenseGameMode` (`GameplayStatics.GetGameMode`)))
  (for _array_element (`self.EnemiesInLineOfFire`)
    (`/Game/TowerDefense/Blueprints/Enemy_Gob.TakeDamage` _array_element (/ (+ (`/Game/TowerDefense/Blueprints/TowerDefenseGameMode.Tower3` _astower_defense_game_mode) 1.0) 2.0))))

(fn `ChangeTarget`
  (bind _enemiesinrange (`self.EnemiesInRange`))
  (`KismetArrayLibrary.Array_RemoveItem` _enemiesinrange (`self.FarthestEnemy`))
  (if (!= (`KismetArrayLibrary.Array_Length` _enemiesinrange) 0)
    (set `self.FarthestEnemy` (`|GetArrayItem` _enemiesinrange (`KismetArrayLibrary.Array_LastIndex` _enemiesinrange)))))

(fn `ChargeUp`
  (bind _output_get (set `self.Charge` (+ (`self.Charge`) 1.0)))
  (if (>= _output_get 50.0)
    (set `self.Charged` true)
    (`KismetSystemLibrary.K2_ClearTimer` null "ChargeUp")
    (else
      (`ParticleSystemComponent.SetTemplate` (`self.LaserEmitter`) null))))

(fn `DeactvateLaser`
  (bind _laseremitter (`self.LaserEmitter`))
  (`ParticleSystemComponent.SetTemplate` _laseremitter null)
  (`SceneComponent.SetVisibility` _laseremitter false true))

(fn `Fire`
  (params (arrow :type "ArrowComponent Object Reference"))
  (bind _returnvalue (`|SpawnActorFromClass` "/Game/TowerDefense/Blueprints/Bullet.Bullet_C" (`SceneComponent.K2_GetComponentToWorld` arrow) "AlwaysSpawn" "OverrideRootScale"))
  (set `/Game/TowerDefense/Blueprints/Bullet.EnemyTarget` (`self.FarthestEnemy`) _returnvalue))

(fn `RotateToTarget`
  (params (Time :type "Float (double-precision)"))
  (returns (`facingTarget?` :type Boolean))
  (bind _turrethead (`self.turretHead`))
  (bind _returnvalue (`SceneComponent.K2_GetComponentRotation` _turrethead))
  (bind _returnvalue_2 (`KismetMathLibrary.FindLookAtRotation` (`self.K2_GetActorLocation`) (`self.K2_GetActorLocation` (`self.FarthestEnemy`))))
  (`SceneComponent.K2_SetWorldRotation` _turrethead (`KismetMathLibrary.RInterpTo` _returnvalue (`KismetMathLibrary.MakeRotator` 0.0 0.0 (+ (.yaw _returnvalue_2) -90.0)) Time (`self.RotationSpeed`)) false false)
  (return (`KismetMathLibrary.NearlyEqual_FloatFloat` (.yaw _returnvalue) (+ (.yaw _returnvalue_2) -90.0) 5.0)))

(fn `UserConstructionScript`)

(fn `ValidAndAlive?`
  (returns (`Targetable?` :type Boolean))
  (locals (RetVal :type Boolean))
  (bind _farthestenemy (`self.FarthestEnemy`))
  (`/Engine/EditorBlueprintResources/StandardMacros.IsValid` _farthestenemy
    (:`Is Valid`
      (set `local.RetVal` (`/Game/TowerDefense/Blueprints/Enemy_Gob.isAlive` _farthestenemy)))
    (:`Is Not Valid`
      (set `local.RetVal` false)))
  (return (`local.RetVal`)))