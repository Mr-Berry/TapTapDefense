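; Goblin-style enemy character for the tower defense game that takes damage and awards fame when killed.
; Damage lowers health and randomly plays a pain sound.
; A one-shot death branch notifies the game mode, disables capsule collision, detaches the controller, plays a random death animation and possible sound, then destroys the actor after a delay.
; SetParamters scales fame by a multiplier and health by the larger of two multipliers.
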(event `self.ReceiveBeginPlay`
  (bind _astower_defense_game_mode (cast `/Game/TowerDefense/Blueprints/TowerDefenseGameMode` (`GameplayStatics.GetGameMode`)))
  (set `self.GameMode` _astower_defense_game_mode))

(event `TakeDamage`
  (params (Damage :type "Float (double-precision)"))
  (bind _mesh (`self.Mesh`))
  (bind _output_get (set `self.Health` (- (`self.Health`) Damage)))
  (bind _output_get_2 (set `self.isAlive` (> _output_get 0.0)))
  (if _output_get_2
    (switch `int` (`KismetMathLibrary.RandomInteger` (`self.SoundChance`))
      (:`0`
        (`GameplayStatics.PlaySoundAtLocation` (`self.PainSound`) (`self.K2_GetActorLocation`))))
    (else
      (`/Engine/EditorBlueprintResources/StandardMacros.DoOnce` false
        (:`Completed`
          (`/Game/TowerDefense/Blueprints/TowerDefenseGameMode.EnemyDeath` (`self.GameMode`) (`self.FameAwarded`))
          (`PrimitiveComponent.SetCollisionEnabled` (`self.CapsuleComponent`) "NoCollision")
          (switch `int` (`KismetMathLibrary.RandomInteger` (`self.SoundChance`))
            (:`Default`
              _)
            (:`0`
              (`GameplayStatics.PlaySoundAtLocation` (`self.DeathSound`) (`self.K2_GetActorLocation`))))
          (`self.DetachFromControllerPendingDestroy`)
          (switch `int` (`KismetMathLibrary.RandomInteger` 3)
            (:`Default`
              (`SkeletalMeshComponent.PlayAnimation` _mesh (`self.Death3`) false))
            (:`0`
              (`SkeletalMeshComponent.PlayAnimation` _mesh (`self.Death1`) false))
            (:`1`
              (`SkeletalMeshComponent.PlayAnimation` _mesh (`self.Death2`) false)))
          (`KismetSystemLibrary.Delay` 2.0)
          (`self.K2_DestroyActor`))))))

(fn `SetParamters`
  (params (Health :type "Float (double-precision)") (FameAwarded :type Integer) (Multiplier :type "Float (double-precision)") (HealthMultiplier :type "Float (double-precision)"))
  (locals (Bonus :type "Float (double-precision)"))
  (bind _returnvalue (* Health Multiplier))
  (bind _returnvalue_2 (* Health HealthMultiplier))
  (set `self.FameAwarded` (`KismetMathLibrary.FTrunc` (* FameAwarded Multiplier)))
  (if (> _returnvalue _returnvalue_2)
    (set `local.Bonus` _returnvalue)
    (else
      (set `local.Bonus` _returnvalue_2)))
  (bind _output_get (set `self.Health` (`local.Bonus`)))
  (set `self.MaxHealth` _output_get))

(fn `UserConstructionScript`)