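; Enemy_Vamp is a vampire enemy Blueprint for the tower defense game, built on a parent enemy class that supplies the behavior.
; On BeginPlay it runs the parent logic, then links its widget's HealthBar to itself.
; It then fills inherited variables with vampire death animations, a death sound, sound chance and fame reward, leaving the pain sound empty.
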(event `self.ReceiveBeginPlay`
  (`parent.ReceiveBeginPlay`)
  (bind _ashealth_bar (cast `/Game/TowerDefense/Interface/HealthBar` (`WidgetComponent.GetUserWidgetObject` (`self.Widget`))))
  (set `/Game/TowerDefense/Interface/HealthBar.Enemy` self _ashealth_bar)
  (set `self.Death1` "/Game/TowerDefense/EnemyAnimations/Vamp_Death_1.Vamp_Death_1")
  (set `self.Death2` "/Game/TowerDefense/EnemyAnimations/Vamp_Death_2.Vamp_Death_2")
  (set `self.Death3` "/Game/TowerDefense/EnemyAnimations/Vamp_Death_3.Vamp_Death_3")
  (set `self.DeathSound` "/Game/TowerDefense/Sounds/death_vamp_Cue.death_vamp_Cue")
  (set `self.PainSound` null)
  (set `self.SoundChance` 5)
  (set `self.FameAwarded` 3))

(fn `UserConstructionScript`
  (`parent.UserConstructionScript`))