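; Tower defense turret that fires AoE bullets at Enemy_Gob targets within its range.
; Range overlaps maintain an enemy list, whose first entry becomes ClosestEnemy without any distance comparison.
; Tick interpolates the head's yaw toward that target and, once nearly aligned, fires on a delay-gated cooldown.
; Each shot spawns a homing-target bullet with optional sound and head recoil, while dead targets are swapped out.
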(event `self.ReceiveTick`
  (params (DeltaSeconds :type "Float (single-precision)"))
  (`/Engine/EditorBlueprintResources/StandardMacros.IsValid` (`self.ClosestEnemy`)
    (:`Is Valid`
      (bind _facingtarget_ (`self.RotateToTarget` DeltaSeconds))
      (if _facingtarget_
        (if (not (`self.isFiring`))
          (set `self.isFiring` true)
          (`self.FireAndKickBack` (`self.Arrow`))
          (`KismetSystemLibrary.Delay` (`self.fireDelay`))
          (set `self.isFiring` false))))))

(event `FireAndKickBack`
  (params (Arrow :type "ArrowComponent Object Reference"))
  (bind _turrethead (`self.TurretHead`))
  (bind _returnvalue (`SceneComponent.GetForwardVector` (`self.Arrow`)))
  (bind _relativerotation (`SceneComponent.RelativeRotation` _turrethead))
  (bind _targetable_ (`self.ValidAndAlive`))
  (if _targetable_
    (`self.Fire` Arrow)
    (`KismetSystemLibrary.MoveComponentTo` _turrethead (* _returnvalue -40) _relativerotation true)
    (`KismetSystemLibrary.MoveComponentTo` _turrethead (* _returnvalue 40) _relativerotation true false 0.3)
    (else
      (`self.ChangeTarget`))))

(event `self.Range.OnComponentBeginOverlap`
  (params (OverlappedComponent :type "PrimitiveComponent Object Reference") (OtherActor :type "Actor Object Reference") (OtherComp :type "PrimitiveComponent Object Reference") (OtherBodyIndex :type Integer) (bFromSweep :type Boolean) (SweepResult :type "HitResult Structure (by ref)"))
  (bind _enemiesinrange (`self.EnemiesInRange`))
  ;[1 1 1] Add enemy to target list when it enters range
  (bind _asenemy_gob (cast `/Game/TowerDefense/Blueprints/Enemy_Gob` OtherActor))
  (set `self.enemyInRange` true)
  (`KismetArrayLibrary.Array_Add` _enemiesinrange _asenemy_gob)
  (set `self.ClosestEnemy` (`|GetArrayItem` _enemiesinrange)))

(event `self.Range.OnComponentEndOverlap`
  (params (OverlappedComponent :type "PrimitiveComponent Object Reference") (OtherActor :type "Actor Object Reference") (OtherComp :type "PrimitiveComponent Object Reference") (OtherBodyIndex :type Integer))
  (bind _enemiesinrange (`self.EnemiesInRange`))
  ;[1 1 1] Remove enemy from target list when it dies/leaves range
  (bind _asenemy_gob (cast `/Game/TowerDefense/Blueprints/Enemy_Gob` OtherActor))
  (`KismetArrayLibrary.Array_RemoveItem` _enemiesinrange _asenemy_gob)
  (set `self.ClosestEnemy` (`|GetArrayItem` _enemiesinrange)))

(fn `ChangeTarget`
  (bind _enemiesinrange (`self.EnemiesInRange`))
  (`KismetArrayLibrary.Array_RemoveItem` _enemiesinrange (`self.ClosestEnemy`))
  (if (!= (`KismetArrayLibrary.Array_Length` _enemiesinrange) 0)
    (set `self.ClosestEnemy` (`|GetArrayItem` _enemiesinrange))))

(fn `Fire`
  (params (arrow :type "ArrowComponent Object Reference"))
  (bind _returnvalue (`|SpawnActorFromClass` "/Game/TowerDefense/Blueprints/AoEBullet.AoEBullet_C" (`SceneComponent.K2_GetComponentToWorld` arrow) "AlwaysSpawn" "OverrideRootScale"))
  (set `/Game/TowerDefense/Blueprints/Bullet.EnemyTarget` (`self.ClosestEnemy`) _returnvalue)
  (if (`self.PlaySound?`)
    (`GameplayStatics.PlaySoundAtLocation` "/Game/TowerDefense/Sounds/AoECan_Cue.AoECan_Cue" (`self.K2_GetActorLocation`))))

(fn `RotateToTarget`
  (params (Time :type "Float (double-precision)"))
  (returns (`facingTarget?` :type Boolean))
  (bind _returnvalue (`SceneComponent.K2_GetComponentRotation` (`self.TurretHead`)))
  (bind _returnvalue_2 (`KismetMathLibrary.FindLookAtRotation` (`self.K2_GetActorLocation`) (`self.K2_GetActorLocation` (`self.ClosestEnemy`))))
  (`SceneComponent.K2_SetWorldRotation` (`self.TurretHead`) (`KismetMathLibrary.RInterpTo` _returnvalue (`KismetMathLibrary.MakeRotator` 0.0 0.0 (+ (.yaw _returnvalue_2) -90.0)) Time (`self.RotationSpeed`)) false false)
  (return (`KismetMathLibrary.NearlyEqual_FloatFloat` (.yaw _returnvalue) (+ (.yaw _returnvalue_2) -90.0) 5.0)))

(fn `UserConstructionScript`)

(fn `ValidAndAlive`
  (returns (`Targetable?` :type Boolean))
  (locals (RetVal :type Boolean))
  (bind _closestenemy (`self.ClosestEnemy`))
  (`/Engine/EditorBlueprintResources/StandardMacros.IsValid` _closestenemy
    (:`Is Valid`
      (set `local.RetVal` (`/Game/TowerDefense/Blueprints/Enemy_Gob.isAlive` _closestenemy)))
    (:`Is Not Valid`
      (set `local.RetVal` false)))
  (return (`local.RetVal`)))