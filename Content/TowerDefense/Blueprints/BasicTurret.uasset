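; Tower defense turret that tracks Enemy_Gob actors entering its range and fires a six-cannon volley at the first one in its list.
; Tick yaws the head toward the target with RInterpTo, starts a volley once aligned within tolerance, and switches target when it is invalid or dead.
; FireAllCannons staggers shots by FireRate, rechecking the target before each.
; Each shot spawns a Bullet given that target, with muzzle flash, optional sound and barrel recoil.
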(event `FireAllCannons`
  (bind _firerate (`self.fireRate`))
  (bind _firerate_2 (`self.fireRate`))
  (set `self.isFiring` true)
  (bind _targetable (`self.ValidAndAlive`))
  (if _targetable
    (`self.FireAndKickBack` (`self.Arrow6`) (`self.turretCannon6`))
    (`KismetSystemLibrary.Delay` _firerate)
    (bind _targetable_2 (`self.ValidAndAlive`))
    (if _targetable_2
      (`self.FireAndKickBack` (`self.Arrow5`) (`self.turretCannon5`))
      (`KismetSystemLibrary.Delay` _firerate)
      (bind _targetable_3 (`self.ValidAndAlive`))
      (if _targetable_3
        (`self.FireAndKickBack` (`self.Arrow4`) (`self.turretCannon4`))
        (`KismetSystemLibrary.Delay` _firerate)
        (bind _targetable_4 (`self.ValidAndAlive`))
        (if _targetable_4
          (`self.FireAndKickBack` (`self.Arrow3`) (`self.turretCannon3`))
          (`KismetSystemLibrary.Delay` _firerate)
          (bind _targetable_5 (`self.ValidAndAlive`))
          (if _targetable_5
            (`self.FireAndKickBack` (`self.Arrow2`) (`self.turretCannon2`))
            (`KismetSystemLibrary.Delay` _firerate)
            (bind _targetable_6 (`self.ValidAndAlive`))
            (if _targetable_6
              (`self.FireAndKickBack` (`self.Arrow1`) (`self.turretCannon1`)))
            (`KismetSystemLibrary.Delay` _firerate)
            (else
              (`KismetSystemLibrary.Delay` (* _firerate_2 2.0))))
          (else
            (`KismetSystemLibrary.Delay` (* _firerate_2 3.0))))
        (else
          (`KismetSystemLibrary.Delay` (* _firerate_2 4.0))))
      (else
        (`KismetSystemLibrary.Delay` (* _firerate_2 5.0))))
    (set `self.isFiring` false)
    (else
      (`KismetSystemLibrary.Delay` (* _firerate_2 6.0)))))

(event `self.ReceiveTick`
  (params (DeltaSeconds :type "Float (single-precision)"))
  (bind _targetable (`self.ValidAndAlive`))
  (if _targetable
    (bind _facingtarget_ (`self.RotateToTarget` DeltaSeconds))
    (if _facingtarget_
      (if (not (`self.isFiring`))
        (`self.FireAllCannons`)))
    (else
      (`self.ChangeTarget`))))

(event `FireAndKickBack`
  (params (Arrow :type "ArrowComponent Object Reference") (Turret :type "StaticMeshComponent Object Reference"))
  (`self.Fire` Arrow)
  (`KismetSystemLibrary.MoveComponentTo` Turret (0.0 -80.0 0.0) (struct) true)
  (`KismetSystemLibrary.MoveComponentTo` Turret (0.0 0.0 0.0) (struct) true false 0.4))

(event `self.Range.OnComponentBeginOverlap`
  (params (OverlappedComponent :type "PrimitiveComponent Object Reference") (OtherActor :type "Actor Object Reference") (OtherComp :type "PrimitiveComponent Object Reference") (OtherBodyIndex :type Integer) (bFromSweep :type Boolean) (SweepResult :type "HitResult Structure (by ref)"))
  (bind _enemiesinrange (`self.EnemiesInRange`))
  ;[1 1 1] Targets in/ targets out
  (bind _asenemy_gob (cast `/Game/TowerDefense/Blueprints/Enemy_Gob` OtherActor))
  (set `self.enemyInRange` true)
  (`KismetArrayLibrary.Array_Add` _enemiesinrange _asenemy_gob)
  (set `self.ClosestEnemy` (`|GetArrayItem` _enemiesinrange)))

(event `self.Range.OnComponentEndOverlap`
  (params (OverlappedComponent :type "PrimitiveComponent Object Reference") (OtherActor :type "Actor Object Reference") (OtherComp :type "PrimitiveComponent Object Reference") (OtherBodyIndex :type Integer))
  (bind _enemiesinrange (`self.EnemiesInRange`))
  ;[1 1 1] Targets in/ targets out
  (bind _asenemy_gob (cast `/Game/TowerDefense/Blueprints/Enemy_Gob` OtherActor))
  (`KismetArrayLibrary.Array_RemoveItem` _enemiesinrange _asenemy_gob)
  (if (!= (`KismetArrayLibrary.Array_Length` _enemiesinrange) 0)
    (set `self.ClosestEnemy` (`|GetArrayItem` _enemiesinrange))
    (else
      (set `self.enemyInRange` false))))

(fn `ChangeTarget`
  (bind _enemiesinrange (`self.EnemiesInRange`))
  (`KismetArrayLibrary.Array_RemoveItem` _enemiesinrange (`self.ClosestEnemy`))
  (if (!= (`KismetArrayLibrary.Array_Length` _enemiesinrange) 0)
    (set `self.ClosestEnemy` (`|GetArrayItem` _enemiesinrange))))

(fn `Fire`
  (params (arrow :type "ArrowComponent Object Reference"))
  (bind _returnvalue (`|SpawnActorFromClass` "/Game/TowerDefense/Blueprints/Bullet.Bullet_C" (`SceneComponent.K2_GetComponentToWorld` arrow) "AlwaysSpawn" "OverrideRootScale"))
  (set `/Game/TowerDefense/Blueprints/Bullet.EnemyTarget` (`self.ClosestEnemy`) _returnvalue)
  (bind _returnvalue_2 (`self.K2_GetActorLocation` _returnvalue))
  (bind _returnvalue_3 (`GameplayStatics.SpawnEmitterAtLocation` "/Game/TowerDefense/Particle/P_BackPack_MuzzleFlash.P_BackPack_MuzzleFlash" _returnvalue_2 (`KismetMathLibrary.MakeRotator` (.roll (`SceneComponent.K2_GetComponentRotation` (`self.turretHead`))) (.pitch (`SceneComponent.K2_GetComponentRotation` (`self.turretHead`))) (+ (.yaw (`SceneComponent.K2_GetComponentRotation` (`self.turretHead`))) 90.0))))
  (`SceneComponent.SetWorldScale3D` _returnvalue_3 (0.2 0.2 0.2))
  (if (`self.PlaySound?`)
    (`GameplayStatics.PlaySoundAtLocation` "/Game/TowerDefense/Sounds/CannonFire_Cue.CannonFire_Cue" _returnvalue_2)))

(fn `RotateToTarget`
  (params (Time :type "Float (double-precision)"))
  (returns (`facingTarget?` :type Boolean))
  (bind _turrethead (`self.turretHead`))
  (bind _returnvalue (`SceneComponent.K2_GetComponentRotation` _turrethead))
  (bind _returnvalue_2 (`KismetMathLibrary.FindLookAtRotation` (`self.K2_GetActorLocation`) (`self.K2_GetActorLocation` (`self.ClosestEnemy`))))
  (`SceneComponent.K2_SetWorldRotation` _turrethead (`KismetMathLibrary.RInterpTo` _returnvalue (`KismetMathLibrary.MakeRotator` 0.0 0.0 (+ (.yaw _returnvalue_2) -90.0)) Time (`self.RotationSpeed`)) false false)
  (return (`KismetMathLibrary.NearlyEqual_FloatFloat` (.yaw _returnvalue) (+ (.yaw _returnvalue_2) -90.0) 5.0)))

(fn `UserConstructionScript`)

(fn `ValidAndAlive`
  (returns (Targetable :type Boolean))
  (locals (RetVal :type Boolean))
  (bind _closestenemy (`self.ClosestEnemy`))
  (`/Engine/EditorBlueprintResources/StandardMacros.IsValid` _closestenemy
    (:`Is Valid`
      (set `local.RetVal` (`/Game/TowerDefense/Blueprints/Enemy_Gob.isAlive` _closestenemy)))
    (:`Is Not Valid`
      (set `local.RetVal` false)))
  (return (`local.RetVal`)))